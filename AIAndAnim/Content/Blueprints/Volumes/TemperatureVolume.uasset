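; TemperatureVolume is a box trigger volume that applies its temperature to characters inside it.
; When an AIAndAnimCharacter with a BPC_HeatSense component begins overlap, it caches that component and starts a one-second looping timer that passes VolumeTemperature to UpdateTemperature.
; It tracks only one actor at a time, and any end overlap clears the timer and cached references.
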(event OnComponentBeginOverlap(Box)
  (params (OverlappedComponent :type Primitive%20Component%20Object%20Reference) (OtherActor :type Actor%20Object%20Reference) (OtherComp :type Primitive%20Component%20Object%20Reference) (OtherBodyIndex :type Integer) (bFromSweep :type Boolean) (SweepResult :type Hit%20Result%20Structure%20%28by%20ref%29))
  (bind _output_get (Variables|Default|SetOverlappingActor OtherActor))
  (if (Utilities|ClassIsChildOf (Utilities|GetClass _output_get) "/Script/AIAndAnim.AIAndAnimCharacter")
    (Utilities|IsValid (Actor|GetComponentbyClass (Variables|Default|GetOverlappingActor) "/Game/Blueprints/Components/BPC_HeatSense.BPC_HeatSense_C")
      (:Is%20Valid
        (Variables|Default|SetOverlappedActorHeatSenseComp (Actor|GetComponentbyClass (Variables|Default|GetOverlappingActor) "/Game/Blueprints/Components/BPC_HeatSense.BPC_HeatSense_C"))
        (Utilities|Time|SetTimerbyFunctionName self "CallUpdateTemperature" 1.0 true)))))

(event OnComponentEndOverlap(Box)
  (params (OverlappedComponent :type Primitive%20Component%20Object%20Reference) (OtherActor :type Actor%20Object%20Reference) (OtherComp :type Primitive%20Component%20Object%20Reference) (OtherBodyIndex :type Integer))
  (Utilities|Time|ClearTimerbyFunctionName self "CallUpdateTemperature")
  (Variables|Default|SetOverlappedActorHeatSenseComp 0)
  (Variables|Default|SetOverlappingActor 0))

(event EventBeginPlay)

(event Collision|EventActorBeginOverlap
  (params (OtherActor :type Actor%20Object%20Reference)))

(event EventTick
  (params (DeltaSeconds :type Float%20%28single-precision%29)))

(fn ConstructionScript)

(fn CallUpdateTemperature
  (bind _overlappedactorheatsensecomp (Variables|Default|GetOverlappedActorHeatSenseComp))
  (Utilities|IsValid _overlappedactorheatsensecomp
    (:Is%20Valid
      (Default|UpdateTemperature _overlappedactorheatsensecomp (Variables|Temperature|GetVolumeTemperature)))))