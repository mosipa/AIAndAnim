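; BPC_HeatSense is a component that tracks a current temperature value for what appears to be its owning actor.
; It sets that value from a starting temperature on BeginPlay.
; UpdateTemperature eases it toward a supplied outside temperature with FInterpTo and world delta time, so each call advances one step.
; Tick only prints the current value on screen as debug output.
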(event EventBeginPlay
  (Variables|Temperature|SetCurrentTemperature (Variables|Temperature|GetStartingTemprature)))

(event EventTick
  (params (DeltaSeconds :type Float%20%28single-precision%29))
  (Development|PrintString (Utilities|String|ToString(Float) (Variables|Temperature|GetCurrentTemperature)) true true "(R=1.000000,G=0.184774,B=0.000000,A=1.000000)" 0.0))

(fn UpdateTemperature
  (params (OutsideTemperature :type Float%20%28single-precision%29))
  (Variables|Temperature|SetCurrentTemperature (Math|Interpolation|FInterpTo (Variables|Temperature|GetCurrentTemperature) OutsideTemperature (Utilities|Time|GetWorldDeltaSeconds) 1.0)))